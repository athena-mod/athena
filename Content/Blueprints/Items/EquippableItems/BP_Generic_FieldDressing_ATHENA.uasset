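; Generic field dressing item that slows the owner's bleeding and limits revives to downed medics.
; Alt use calls BandagedBleed on the owner after a retriggerable delay if still in progress, or only shows a message if already bandaged.
; Use sphere-traces from the first-person camera socket and casts through four faction medic classes.
; It cancels on living, non-bleeding medics and on downed non-medics, messaging the player for the latter.
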(event EventBPBeginUse
  ;[1 1 1] Calculate Interaction Vector from camera socket <Courtesy of OWI from BP_GenericShovel with slight modifications>
  (bind _asbp_mutable_soldier_child_athena (Utilities|Casting|CastToBP_MutableSoldier_Child_ATHENA (Components|GetOwner)))
  (if (Utilities|IsValid _asbp_mutable_soldier_child_athena)
    (bind (_outhit _returnvalue) (Collision|SphereTraceForObjects (Transformation|GetSocketLocation (Variables|/Script/Squad.SQSoldierNew|GetUpperMesh1P _asbp_mutable_soldier_child_athena) "Bip01_CameraBoneSocket") (+ (Transformation|GetSocketLocation (Variables|/Script/Squad.SQSoldierNew|GetUpperMesh1P _asbp_mutable_soldier_child_athena) "Bip01_CameraBoneSocket") (* (Math|Rotator|GetRotationXVector (.OutRotation (Actor|GetActorEyesViewPoint _asbp_mutable_soldier_child_athena))) (Variables|Default|GetTraceLength))) (+ (Variables|Default|GetTraceSphereRadius) 75.0) (Utilities|Array|MakeArray "ObjectTypeQuery3") false (Utilities|Array|MakeArray (Components|GetOwner)) "None"))
    (if _returnvalue
      (bind _asbp_soldier_gb_medic_athena (Utilities|Casting|CastToBP_Soldier_GB_Medic_ATHENA (.HitActor (Collision|BreakHitResult _outhit)))
        (:then
          (if (> (Variables|/Script/Squad.SQSoldier|GetHealth _asbp_soldier_gb_medic_athena) 0.0)
            (if (not (Variables|/Script/Squad.SQSoldier|GetbIsBleeding _asbp_soldier_gb_medic_athena))
              (Class|SQEquipableItem|EndUse))))
        (:CastFailed
          (bind _asbp_soldier_mil_medic_athena (Utilities|Casting|CastToBP_Soldier_MIL_Medic_ATHENA (.HitActor (Collision|BreakHitResult _outhit)))
            (:then
              (if (> (Variables|/Script/Squad.SQSoldier|GetHealth _asbp_soldier_mil_medic_athena) 0.0)
                (if (not (Variables|/Script/Squad.SQSoldier|GetbIsBleeding _asbp_soldier_mil_medic_athena))
                  (Class|SQEquipableItem|EndUse))))
            (:CastFailed
              (bind _asbp_soldier_usa_medic_athena (Utilities|Casting|CastToBP_Soldier_USA_Medic_ATHENA (.HitActor (Collision|BreakHitResult _outhit)))
                (:then
                  (if (> (Variables|/Script/Squad.SQSoldier|GetHealth _asbp_soldier_usa_medic_athena) 0.0)
                    (if (not (Variables|/Script/Squad.SQSoldier|GetbIsBleeding _asbp_soldier_usa_medic_athena))
                      (Class|SQEquipableItem|EndUse))))
                (:CastFailed
                  (bind _asbp_soldier_ru_medic_athena (Utilities|Casting|CastToBP_Soldier_RU_Medic_ATHENA (.HitActor (Collision|BreakHitResult _outhit)))
                    (:then
                      (if (> (Variables|/Script/Squad.SQSoldier|GetHealth _asbp_soldier_ru_medic_athena) 0.0)
                        (if (not (Variables|/Script/Squad.SQSoldier|GetbIsBleeding _asbp_soldier_ru_medic_athena))
                          (Class|SQEquipableItem|EndUse))))
                    (:CastFailed
                      (bind _asbp_mutable_soldier_child_athena_2 (Utilities|Casting|CastToBP_MutableSoldier_Child_ATHENA (.HitActor (Collision|BreakHitResult _outhit))))
                      (if (not (> (Variables|/Script/Squad.SQSoldier|GetHealth _asbp_mutable_soldier_child_athena_2) 0.0))
                        (Class|SQEquipableItem|EndUse)
                        (bind _assqsoldier_new (Utilities|Casting|CastToSQSoldierNew (Components|GetOwner)))
                        (bind _assqplayer_controller (Utilities|Casting|CastToSQPlayerController (Pawn|GetController _assqsoldier_new)))
                        (Class|SQPlayerController|ClientSystemMessage _assqplayer_controller "You can only revive other medics" (Math|Color|MakeColor 0.0 0.0 0.0) -1.0 "Negative")))))))))))))

(event EventBPBeginAltUse
  (bind _asbp_mutable_soldier_child_athena (Utilities|Casting|CastToBP_MutableSoldier_Child_ATHENA (Components|GetOwner)))
  (if (Variables|/ATHENA/Blueprints/Soldiers/BP_MutableSoldier_Child_ATHENA.BP_MutableSoldier_Child_ATHENA_C|GetisBandagedBleeding _asbp_mutable_soldier_child_athena)
    (bind _asbp_player_controller_child_athena (Utilities|Casting|CastToBP_PlayerController_Child_ATHENA (Pawn|GetController _asbp_mutable_soldier_child_athena)))
    (Class|SQPlayerController|ClientSystemMessage _asbp_player_controller_child_athena "You are already bandaged, seek medic for further assistance" (Math|Color|MakeColor 0.0 0.0 0.0) -1.0 "Message")
    (else
      (Utilities|FlowControl|RetriggerableDelay 7.2)
      (if (Utilities|Enum|Equal(Enum) (Variables|Default|GetActionState) "AltUse")
        (Default|BandagedBleed _asbp_mutable_soldier_child_athena)
        (bind _asbp_player_controller_child_athena_2 (Utilities|Casting|CastToBP_PlayerController_Child_ATHENA (Pawn|GetController _asbp_mutable_soldier_child_athena)))
        (Class|SQPlayerController|ClientSystemMessage _asbp_player_controller_child_athena_2 "You have have slowed down the bleeding, seek medic for full treatment" (Math|Color|MakeColor 0.0 0.0 0.0) -1.0 "Warning")))))

(fn ConstructionScript)