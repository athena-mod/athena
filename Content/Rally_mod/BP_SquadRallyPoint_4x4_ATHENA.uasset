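; Squad rally point actor that removes itself when no friendly HAB or capture zone is nearby.
; After a one-minute delay, BeginPlay runs a minute-interval loop of 600 m sphere overlaps, comparing team IDs to set a flag.
; A custom delayed for-loop macro breaks when the flag stays unset, and its completion destroys the actor.
; Prompt events add it to same-team players' HUD line-of-sight actors and remove it on hide.
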(event EventBeginPlay
  (Variables|Default|Setflag 0)
  (Utilities|FlowControl|Delay 6e+01)
  (Utilities|ForLoopwithBreakwithDelay 1 99999 6e+01 :!label _label
    (:Loop%20Body
      (bind (_outactors _returnvalue) (Collision|SphereOverlapActors (.OutLocation (Actor|GetActorEyesViewPoint)) 6e+04 (Utilities|Array|MakeArray "ObjectTypeQuery2" "ObjectTypeQuery1") "/Game/Gameplay/Deployables/BP_Deployable_Hab.BP_Deployable_Hab_C"))
      (if _returnvalue
        (for _array_element _outactors
          (bind _returnvalue_2 (Class|SQTeamInterface|GetTeamId(Message) _array_element))
          (bind _returnvalue_3 (Class|SQUsable|GetInterfaceTeam))
          (if (== _returnvalue_2 _returnvalue_3)
            (Variables|Default|Setflag 1))))
      (bind _returnvalue_4 (Collision|SphereOverlapActors (.OutLocation (Actor|GetActorEyesViewPoint)) 6e+04 (Utilities|Array|MakeArray "ObjectTypeQuery1" "ObjectTypeQuery2" "ObjectTypeQuery8" "ObjectTypeQuery10") "/Game/Blueprints/Placeable/CaptureZones/BP_CaptureZone.BP_CaptureZone_C"))
      (if _returnvalue_4
        (for _array_element_2 0
          (bind _returnvalue_5 (Class|SQTeamInterface|GetTeamId(Message) _array_element_2))
          (bind _returnvalue_6 (Class|SQUsable|GetInterfaceTeam))
          (if (== _returnvalue_5 _returnvalue_6)
            (Variables|Default|Setflag 1))))
      (if (== (Variables|Default|Getflag) 0)
        (goto _label Break)
        (else
          (Variables|Default|Setflag 0))))
    (:Completed
      (Actor|DestroyActor))))

(event EventBPHidePrompt
  (bind _return_value (CallFunction|GetSquadPlayerController))
  (Utilities|IsValid _return_value
    (:Is%20Valid
      (bind _assqhud (Utilities|Casting|CastToSQHUD (HUD|GetHUD _return_value)))
      (Class|SQHUD|RemoveLineOfSightActor _assqhud self))))

(event EventBPDisplayPrompt
  (params (User :type Controller%20Object%20Reference))
  (bind _assqplayer_controller (Utilities|Casting|CastToSQPlayerController User))
  (if (== (Class|SQPlayerController|GetTeam _assqplayer_controller) (Math|Conversions|ToInteger(Byte) (Variables|Default|GetTeam)))
    (bind _assqhud (Utilities|Casting|CastToSQHUD (HUD|GetHUD _assqplayer_controller)))
    (Class|SQHUD|AddLineOfSightActor _assqhud self)))

(fn ConstructionScript)

(fn GetInterfaceTeam
  (return (Math|Conversions|ToInteger(Byte) (Class|SQGameSpawn|GetTeam))))

(fn GetUsableData
  (return (Variables|Default|GetData)))