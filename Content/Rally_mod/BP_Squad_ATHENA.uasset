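; Squad Blueprint for the Rally mod that sends membership notifications to players and cleans up the squad's map markers.
; On authority, it binds squad events to client notifications for leaders on joins (via the misnamed OnLeaveEvent), departures and promotions, and for each updated non-Alpha fireteam's first member.
; Fireteam updates and disbands remove markers of emptied fireteams, clearing all fireteam markers when no non-Alpha members remain.
; Destruction removes every tracked marker.
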(event Custom|OnFireteamDisbanded_Event_0
  (params (Squad :type SQ%20Squad%20Object%20Reference) (FireteamID :type Integer))
  (CallFunction|DestroyFireteamMarkers FireteamID))

(event Custom|OnPlayerJoinSquad_Event_0
  (params (Squad :type SQ%20Squad%20Object%20Reference) (Player :type SQ%20Player%20Controller%20Object%20Reference))
  (CallFunction|OnLeaveEvent Squad Player))

(event Custom|OnFireteamUpdated_Event_0
  (params (Squad :type SQ%20Squad%20Object%20Reference) (FireteamID :type Integer))
  (CallFunction|DestroyFireteamMarkers FireteamID)
  (CallFunction|FireteamNotification Squad FireteamID))

(event Custom|OnPlayerPartSquad_Event_0
  (params (Squad :type SQ%20Squad%20Object%20Reference) (Player :type SQ%20Player%20Controller%20Object%20Reference))
  (CallFunction|PartingNotification Squad Player))

(event Custom|OnPlayerBecomeSquadLeader_Event_0
  (params (Squad :type SQ%20Squad%20Object%20Reference) (Player :type SQ%20Player%20Controller%20Object%20Reference))
  (CallFunction|BecomeSLNotification Squad))

(event EventBeginPlay
  (Networking|SwitchHasAuthority
    (:Authority
      (EventDispatchers|AssignOnFireteamDisbanded (delegate Custom|OnFireteamDisbanded_Event_0))
      (EventDispatchers|AssignOnFireteamUpdated (delegate Custom|OnFireteamUpdated_Event_0))
      (Utilities|FlowControl|Sequence
        (:then_0
          (EventDispatchers|AssignOnPlayerPartSquad (delegate Custom|OnPlayerPartSquad_Event_0)))
        (:then_1
          (EventDispatchers|AssignOnPlayerJoinSquad (delegate Custom|OnPlayerJoinSquad_Event_0)))
        (:then_2
          (EventDispatchers|AssignOnPlayerBecomeSquadLeader (delegate Custom|OnPlayerBecomeSquadLeader_Event_0)))))))

(event EventDestroyed
  (CallFunction|DestroyAllMarkers))

(fn ConstructionScript)

(fn DestroyAllMarkers
  (Utilities|FlowControl|Sequence
    (:then_0
      (LocalVariables|SetMarkers%20To%20Destroy (Variables|Default|GetLatestActionMarkers))
      (Utilities|Array|AppendArray (LocalVariables|GetMarkers%20To%20Destroy) (Variables|Default|GetLatestFireteamMarkers))
      (Utilities|Array|AppendArray (LocalVariables|GetMarkers%20To%20Destroy) (Variables|Default|GetLatestPOIMarkers))
      (Utilities|Array|AppendArray (LocalVariables|GetMarkers%20To%20Destroy) (Variables|Default|GetLatestRequestMarkers))
      (Utilities|Array|AppendArray (LocalVariables|GetMarkers%20To%20Destroy) (Variables|Default|GetLatestSpotMarkers)))
    (:then_1
      (for _array_element (LocalVariables|GetMarkers%20To%20Destroy)
        (Utilities|IsValid _array_element
          (:Is%20Valid
            (Actor|DestroyActor _array_element)))))))

(fn DestroyFireteamMarkers
  (params (ID :type Integer))
  (bind _latestfireteammarkers (Variables|Default|GetLatestFireteamMarkers))
  (bind _fireteams (Variables|Default|GetFireTeams))
  (if (Utilities|Array|IsValidIndex _fireteams ID)
    (if (== (Utilities|Array|Length (.players (Utilities|Array|Get(acopy) _fireteams ID))) 0)
      (for _array_element (Variables|Default|GetLatestFireteamMarkers)
        (if (== (Class|SQMapMarker|GetFireteamId _array_element) ID)
          (Actor|DestroyActor _array_element)
          (Utilities|Array|RemoveItem (Variables|Default|GetLatestFireteamMarkers) _array_element)))
      (for (_array_element_2 _array_index) (Variables|Default|GetFireTeams)
        (if (> _array_index 0)
          (if (>= (Utilities|Array|Length (Utilities|Struct|BreakSQFireTeam _array_element_2)) 1)
            (LocalVariables|SetHas%20FT%20Members%20in%20other%20squads true))))
      (if (not (LocalVariables|GetHas%20FT%20Members%20in%20other%20squads))
        (for _array_element_3 _latestfireteammarkers
          (Actor|DestroyActor _array_element_3))
        (Utilities|Array|Clear _latestfireteammarkers)))))

(fn FireteamNotification
  (params (Squad :type SQ%20Squad%20Object%20Reference) (FT :type Integer))
  (bind _fireteams (Variables|/Script/Squad.SQSquad|GetFireTeams Squad))
  (bind _output (Utilities|Array|Get(acopy) _fireteams FT))
  (if (!= FT 0) ; ignore alpha
    (if (Utilities|Array|IsValidIndex _fireteams)
      (if (Utilities|Array|IsValidIndex (.players _output))
        (bind _asbp_player_controller (Utilities|Casting|CastToBP_PlayerController (Utilities|Array|Get(acopy) (.players _output))))
        (Default|ClientNotification _asbp_player_controller (Utilities|Text|FormatText "Fireteam {FT} has been updated." (Utilities|Select :Index FT :Option%200 "" :Option%201 "Bravo" :Option%202 "Charlie" :Option%203 "Delta")) "Fireteam")))))

(fn PartingNotification
  (params (Squad :type SQ%20Squad%20Object%20Reference) (Leaving%20State :type Controller%20Object%20Reference))
  (bind _leader (Variables|/Script/Squad.SQSquad|GetLeader Squad)
    (:then
      (bind _asbp_player_controller (Utilities|Casting|CastToBP_PlayerController _leader))
      (bind _assqplayer_state (Utilities|Casting|CastToSQPlayerState (Variables|/Script/Engine.Controller|GetPlayerState Leaving%20State)))
      (Default|ClientNotification _asbp_player_controller (Utilities|Text|FormatText "{name} {text}" (Utilities|Text|ToText(String) (Class|SQPlayerState|GetFullPlayerName _assqplayer_state)) (Utilities|Text|MakeLiteralText " has left the Squad.")) "Squad"))
    (:else)))

(fn BecomeSLNotification
  (params (State :type SQ%20Squad%20Object%20Reference))
  ;[1 1 1] Notify of promotion to SL or Commander
  (bind _leader (Variables|/Script/Squad.SQSquad|GetLeader State)
    (:then
      (bind _asbp_player_controller (Utilities|Casting|CastToBP_PlayerController _leader))
      (if (Class|SQPlayerController|IsCommander _asbp_player_controller)
        (Default|ClientNotification _asbp_player_controller "You have been promoted to Commander." "Commander")
        (else
          (Default|ClientNotification _asbp_player_controller "You have been promoted to Squad Leader." "Squad"))))
    (:else)))

(fn OnLeaveEvent
  (params (Squad :type SQ%20Squad%20Object%20Reference) (Joining%20State :type Controller%20Object%20Reference))
  (bind _leader (Variables|/Script/Squad.SQSquad|GetLeader Squad)
    (:then
      (if (not (== _leader Joining%20State))
        (bind _assqplayer_state (Utilities|Casting|CastToSQPlayerState (Variables|/Script/Engine.Controller|GetPlayerState Joining%20State)))
        (bind _asbp_player_controller (Utilities|Casting|CastToBP_PlayerController _leader))
        (Default|ClientNotification _asbp_player_controller (Utilities|Text|FormatText "{name} {text}" (Utilities|Text|ToText(String) (Class|SQPlayerState|GetFullPlayerName _assqplayer_state)) (Utilities|Text|MakeLiteralText "has joined the Squad.")) "Squad")))
    (:else)))